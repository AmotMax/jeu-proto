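; ChasedAI is an AI-moved pawn that flees from the player's ThirdPersonCharacter when it comes within MinDistance.
; Tick checks the distance to the cached player reference, printing it whenever no escape is triggered.
; RunAway projects a point directly away from the player, then moves to a random reachable navigation point around it.
; A CanEscape flag blocks new escapes until that move succeeds or fails.
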(event `self.ReceiveTick`
  (params (DeltaSeconds :type "Float (single-precision)"))
  (bind _returnvalue (`KismetMathLibrary.Vector_Distance` (`self.K2_GetActorLocation`) (`self.K2_GetActorLocation` (`self.Character Reference`))))
  (if (and (< _returnvalue (`self.MinDistance`)) (`self.CanEscape`))
    (`self.RunAway`)
    (else
      (`KismetSystemLibrary.PrintString` (`KismetStringLibrary.Conv_DoubleToString` _returnvalue)))))

(event `self.ReceiveBeginPlay`
  (bind _asthird_person_character (cast `/Game/ThirdPersonBP/Blueprints/ThirdPersonCharacter` (`GameplayStatics.GetPlayerCharacter` 0)))
  (set `self.Character Reference` _asthird_person_character))

(event `RunAway`
  (bind _returnvalue (`self.K2_GetActorLocation`))
  (set `self.CanEscape` false)
  (`|AIMoveTo` self (`NavigationSystemV1.K2_GetRandomReachablePointInRadius` (`KismetMathLibrary.MakeVector` (.x (+ _returnvalue (* (`KismetMathLibrary.GetForwardVector` (`KismetMathLibrary.FindLookAtRotation` _returnvalue (`self.K2_GetActorLocation` (`self.Character Reference`)))) -500.0))) (.y (+ _returnvalue (* (`KismetMathLibrary.GetForwardVector` (`KismetMathLibrary.FindLookAtRotation` _returnvalue (`self.K2_GetActorLocation` (`self.Character Reference`)))) -500.0))) (.z _returnvalue)) 500.0 null null) null
    (:`OnSuccess`
      _)
    (:`OnFail`
      _))
  (set `self.CanEscape` true))

(fn `UserConstructionScript`)